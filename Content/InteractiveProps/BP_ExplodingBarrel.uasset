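; BP_ExplodingBarrel is an interactive prop that explodes when its HitInteraction event is called.
; The explosion fires a RadialForce impulse, plays a loud sound and spawns a particle effect at the barrel's location.
; It then awards "Explosion!" style points to the player's ThirdPersonCharacter, regardless of who triggered it.
; Afterward, only the Cylinder component is destroyed, so the actor itself remains.
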(event Custom|Explode
  (bind _returnvalue (Transformation|GetActorLocation))
  (Class|RadialForceComponent|FireImpulse (Variables|Default|GetRadialForce))
  (Audio|PlaySoundatLocation "/Game/Sounds/Explosion.Explosion" _returnvalue "0, 0, 0" 3.0 1.0 0.0 0 0 0)
  (Effects|SpawnEmitteratLocation "/Game/Realistic_Starter_VFX_Pack_Vol2/Particles/Explosion/P_Explosion_Big_A.P_Explosion_Big_A" _returnvalue)
  (bind _asthird_person_character (Utilities|Casting|CastToThirdPersonCharacter (Game|GetPlayerCharacter 0)))
  (Default|AddStylePoints _asthird_person_character "Explosion!" 50))

(event EventHitInteraction
  (params (Interactor :type Character%20Object%20Reference))
  (CallFunction|Explode)
  (Components|DestroyComponent (Variables|Default|GetCylinder)))

(fn ConstructionScript)