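; BP_Car is an interactive car prop that moves along a spline and awards style points when it hits the player.
; On BeginPlay, the Cycle timeline plays at a rate set by SpeedTimePerRevolution.
; Its PathProgress drives spline distance, and the sampled local-space location and rotation are applied directly as the actor's transform.
; A Hit with the player pawn casts it to ThirdPersonCharacter and grants "C(h)a(i)r Accident" points.
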(event Custom|MoveObject
  (bind _spline (Variables|Default|GetSpline))
  (Components|Timeline|SetPlayRate (Variables|Default|GetCycle) (/ 1.0 (Variables|Default|GetSpeed%28TimePerRevolution%29)))
  (bind _pathprogress (Timeline|Cycle Play)
    (:Update
      (Transformation|SetActorLocationAndRotation (Spline|GetLocationatDistanceAlongSpline _spline (Math|Float|Lerp 0.0 (Spline|GetSplineLength (Variables|Default|GetSpline)) _pathprogress) "Local") (Spline|GetRotationatDistanceAlongSpline _spline (Math|Float|Lerp 0.0 (Spline|GetSplineLength (Variables|Default|GetSpline)) _pathprogress) "Local")))))

(event EventBeginPlay
  (CallFunction|MoveObject))

(event Collision|EventHit
  (params (MyComp :type Primitive%20Component%20Object%20Reference) (Other :type Actor%20Object%20Reference) (OtherComp :type Primitive%20Component%20Object%20Reference) (bSelfMoved :type Boolean) (HitLocation :type Vector :default "0, 0, 0") (HitNormal :type Vector :default "0, 0, 0") (NormalImpulse :type Vector :default "0, 0, 0") (Hit :type Hit%20Result%20Structure%20%28by%20ref%29))
  (bind _returnvalue (Game|Player|GetPlayerPawn 0))
  (if (== Other _returnvalue)
    (bind _asthird_person_character (Utilities|Casting|CastToThirdPersonCharacter _returnvalue))
    (Default|AddStylePoints _asthird_person_character "C(h)a(i)r Accident" 25)))

(fn ConstructionScript)