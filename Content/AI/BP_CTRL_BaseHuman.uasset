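; AI controller for human NPCs that grow suspicious of the player's chair and flee when they see it move too much.
; It runs BT_BaseHuman while sight perception and Tick logic drive the blackboard state, target location and facial expression.
; Visible player movement builds ChairExposure; crossing the threshold triggers fleeing and "Chair Jumpscare" style points.
; DoOnce gates and retriggerable delays pace the reactions and later exposure reset.
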(event OnTargetPerceptionUpdated(AIPerception)
  (params (Actor :type Actor%20Object%20Reference) (Stimulus :type AI%20Stimulus%20Structure))
  (bind _bsuccessfullysensed (Utilities|Struct|BreakAIStimulus Stimulus))
  (bind _returnvalue (Class|AIPerceptionSystem|GetSenseClassforStimulus Stimulus))
  (if (and (== _returnvalue "/Script/AIModule.AISense_Sight") (== Actor (Game|Player|GetPlayerPawn 0)))
    (if (Variables|Default|GetRunningAwayFromChair)
      (Variables|Default|SetSeeingChair _bsuccessfullysensed)
      (Utilities|FlowControl|DoOnce false) ; enters at Reset
      (else
        (CallFunction|SetBlackboardKeyEnum "State" (select _bsuccessfullysensed 2 1))
        (Variables|Default|SetSeeingChair _bsuccessfullysensed)))))

(event EventBeginPlay
  (AI|RunBehaviorTree "/Game/AI/BT_BaseHuman.BT_BaseHuman")
  (CallFunction|SetBlackboardKeyEnum "State" 1)
  (AI|Components|Blackboard|SetValueasObject (Variables|Default|GetBlackboard) (Utilities|Name|MakeLiteralName "Chair") (Game|Player|GetPlayerPawn 0))
  (bind _asbp_ai_base_human (Utilities|Casting|CastToBP_AI_BaseHuman (Pawn|GetControlledPawn)))
  (Variables|Default|SetControlledHuman _asbp_ai_base_human)
  (Variables|/Game/AI/BP_AI_BaseHuman.BP_AI_BaseHuman_C|SetFacialExpression (Variables|Default|GetControlledHuman) "/Game/Textures/Expressions/STATE_Neutral.STATE_Neutral"))

(event EventTick
  (params (DeltaSeconds :type Float%20%28single-precision%29))
  (bind _returnvalue (CallFunction|GetBlackboardKeyEnum "State"))
  (if (> (Variables|/Game/AI/BP_AI_BaseHuman.BP_AI_BaseHuman_C|GetHP (Variables|Default|GetControlledHuman)) 0.0)
    (if (Variables|Default|GetSeeingChair)
      (Utilities|FlowControl|Sequence
        (:then_0
          (Utilities|FlowControl|DoOnce false :!label _label
            (:Completed
              (CallFunction|SetBlackboardKeyEnum "State")
              (Variables|/Game/AI/BP_AI_BaseHuman.BP_AI_BaseHuman_C|SetFacialExpression (Variables|Default|GetControlledHuman) "/Game/Textures/Expressions/STATE_Attention.STATE_Attention")
              (Utilities|FlowControl|RetriggerableDelay 1.0)
              (Variables|/Game/AI/BP_AI_BaseHuman.BP_AI_BaseHuman_C|SetFacialExpression (Variables|Default|GetControlledHuman) "/Game/Textures/Expressions/STATE_Suspicious.STATE_Suspicious")
              (Utilities|FlowControl|RetriggerableDelay (Math|Random|RandomFloatinRange 5.0 7.0))
              (if (> (Variables|Default|GetChairExposure) 2e+02)
                (Utilities|FlowControl|DoOnce false :!label _label_2
                  (:Completed
                    (Utilities|FlowControl|Sequence
                      (:then_0
                        (Utilities|FlowControl|RetriggerableDelay 15.0)
                        (CallFunction|SetBlackboardKeyEnum "State" 1)
                        (Variables|Default|SetChairExposure 0.0)
                        (goto _label_3 Reset))
                      (:then_1
                        (Utilities|FlowControl|DoOnce false :!label _label_3
                          (:Completed
                            (bind _asthird_person_character (Utilities|Casting|CastToThirdPersonCharacter (Game|GetPlayerCharacter 0)))
                            (Default|AddStylePoints _asthird_person_character "Chair Jumpscare" 5)))))))
                (else
                  (CallFunction|SetBlackboardKeyEnum "State" (select (Math|Random|RandomBoolwithWeight 0.2) 2 1))
                  (Variables|/Game/AI/BP_AI_BaseHuman.BP_AI_BaseHuman_C|SetFacialExpression (Variables|Default|GetControlledHuman) "/Game/Textures/Expressions/STATE_Neutral.STATE_Neutral"))))))
        (:then_1
          (CallFunction|SetBlackboardKeyVector "DesiredLocation" (Transformation|GetActorLocation (Game|Player|GetPlayerPawn 0))))
        (:then_2
          (if (and (Variables|/Game/ThirdPersonBP/Blueprints/ThirdPersonCharacter.ThirdPersonCharacter_C|GetIsMoving (.AsThird%20Person%20Character (Utilities|Casting|CastToThirdPersonCharacter (Game|Player|GetPlayerPawn 0)))) (Math|Boolean|ORBoolean (== _returnvalue 0) (== _returnvalue 1) (== _returnvalue 2)))
            (Utilities|FlowControl|Sequence
              (:then_0
                (bind _output_get (Variables|Default|SetChairExposure (+ (Variables|Default|GetChairExposure) 1.0)))
                (Development|PrintString (Utilities|String|ToString(Float) _output_get))
                (if (> _output_get 2e+02)
                  (CallFunction|SetBlackboardKeyEnum "State" 5)
                  (Variables|Default|SetRunningAwayFromChair true)
                  (goto _label_2 Reset)))
              (:then_1
                (if (not (> _output_get 2e+02))
                  (goto _label Reset)))
              (:then_2
                (goto _label))))))
      (elif (Variables|Default|GetRunningAwayFromChair)
        (Utilities|FlowControl|Sequence
          (:then_0
            (goto _label_2))
          (:then_1
            (CallFunction|SetBlackboardKeyEnum "State" 5)
            (Variables|/Game/AI/BP_AI_BaseHuman.BP_AI_BaseHuman_C|SetFacialExpression (Variables|Default|GetControlledHuman) "/Game/Textures/Expressions/STATE_Scared.STATE_Scared")))
        (else
          (Variables|/Game/AI/BP_AI_BaseHuman.BP_AI_BaseHuman_C|SetFacialExpression (Variables|Default|GetControlledHuman) "/Game/Textures/Expressions/STATE_Neutral.STATE_Neutral"))))
    (else
      (AI|RunBehaviorTree))))

(fn ConstructionScript)

(fn SetBlackboardKeyEnum
  (params (KeyName :type Name) (EnumValue :type Byte))
  (AI|Components|Blackboard|SetValueasEnum (Variables|Default|GetBlackboard) KeyName EnumValue))

(fn SetBlackboardKeyVector
  (params (KeyName :type Name) (VectorValue :type Vector))
  (AI|Components|Blackboard|SetValueasVector (Variables|Default|GetBlackboard) KeyName VectorValue))

(fn GetBlackboardKeyBool
  (params (KeyName :type Name))
  (return (ScalableFloat|GetValueasBool (Variables|Default|GetBlackboard) KeyName)))

(fn GetBlackboardKeyEnum
  (params (KeyName :type Name))
  (return (Class|BlackboardComponent|GetValueasEnum (Variables|Default|GetBlackboard) KeyName)))