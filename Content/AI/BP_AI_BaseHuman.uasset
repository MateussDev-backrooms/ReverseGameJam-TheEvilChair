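; Base human AI character with HP, a billboard face sprite and style-point rewards for the player.
; Hit interactions subtract a fixed amount of HP and AnyDamage subtracts the damage dealt, with any exploding-barrel damage awarding "Boom kill!" points, lethal or not.
; Tick polls HP, showing the facial expression while alive, then running death once: movement and capsule collision stop, the mesh ragdolls, the dead sprite appears and kill points are awarded.
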(event EventTick
  (params (DeltaSeconds :type Float%20%28single-precision%29))
  (if (> (Variables|Default|GetHP) 0.0)
    (Rendering|Components|Sprite|SetSprite (Variables|Default|GetBillboard) (Variables|Default|GetFacialExpression))
    (else
      (Utilities|FlowControl|DoOnce false
        (:Completed
          (Collision|SetCollisionEnabled (Variables|Collision|GetCapsuleComponent) "NoCollision")
          (Pawn|Components|CharacterMovement|SetMovementMode (Variables|Character|GetCharacterMovement) "MOVE_None" 0)
          (Collision|SetCollisionEnabled (Variables|Character|GetMesh) "QueryAndPhysics")
          (Physics|SetSimulatePhysics (Variables|Character|GetMesh) true)
          (Rendering|Components|Sprite|SetSprite (Variables|Default|GetBillboard) "/Game/Textures/Expressions/STATE_Dead.STATE_Dead")
          (Components|Animation|SetAnimationMode (Variables|Character|GetMesh) "AnimationCustomMode")
          (bind _asthird_person_character (Utilities|Casting|CastToThirdPersonCharacter (Game|GetPlayerCharacter 0)))
          (Default|AddStylePoints _asthird_person_character "KILL" 100))))))

(event EventHitInteraction
  (params (Interactor :type Character%20Object%20Reference))
  (Variables|Default|SetHP (- (Variables|Default|GetHP) 1e+01)))

(event Game|Damage|EventAnyDamage
  (params (Damage :type Float%20%28single-precision%29) (DamageType :type Damage%20Type%20Object%20Reference) (InstigatedBy :type Controller%20Object%20Reference) (DamageCauser :type Actor%20Object%20Reference))
  (Variables|Default|SetHP (- (Variables|Default|GetHP) Damage))
  (if (== (Utilities|GetClass DamageCauser) "/Game/InteractiveProps/BP_ExplodingBarrel.BP_ExplodingBarrel_C")
    (bind _asthird_person_character (Utilities|Casting|CastToThirdPersonCharacter (Game|GetPlayerCharacter 0)))
    (Default|AddStylePoints _asthird_person_character "Boom kill!" 150)))

(fn ConstructionScript)